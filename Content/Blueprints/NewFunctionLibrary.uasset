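; Blueprint function library with two input helpers: one for applying rotation to a player controller, one for stick-style deadzone filtering.
; AddInputRotation feeds a rotation's pitch, yaw and roll into the controller's matching input calls.
; CalculateCircularDeadzone compares squared 2D length to the squared threshold, zeroing vectors at or inside it.
; Vectors outside pass through, or optionally get the threshold subtracted per component and are divided by the remaining range.
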(fn AddInputRotation
  (params (PlayerController :type Player%20Controller%20Object%20Reference) (Rotation :type Rotator))
  (Class|PlayerController|AddPitchInput PlayerController (.pitch Rotation))
  (Class|PlayerController|AddYawInput PlayerController (.yaw Rotation))
  (Class|PlayerController|AddRollInput PlayerController (.roll Rotation)))

(fn CalculateCircularDeadzone
  (params (Vector :type Vector%202D%20Structure) (Deadzione :type Float%20%28single-precision%29 :default 0.0) (Scaled? :type Boolean :default false))
  (Math|Float|CompareFloat (Class|KismetMathLibrary|VSize2DSquared Vector) (Math|Float|Square Deadzione)
    (:>
      (if Scaled?
        ;[1 1 1] Scaled Deadzone
        (LocalVariables|SetTemp%20Result (/ (- Vector Deadzione) (- 1.0 Deadzione)))
        (else
          (LocalVariables|SetTemp%20Result Vector))))
    (:==
      (LocalVariables|SetTemp%20Result "" :!label _label))
    (:<
      (goto _label)))
  (return (LocalVariables|GetTemp%20Result)))