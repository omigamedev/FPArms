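; First-person player controller that turns input into camera look, pawn movement and main attacks.
; LookUp and TurnRight axes add pitch and yaw directly, while Tick applies rate-based look scaled by delta time and feeds movement to the pawn, both through scaled circular deadzones.
; Movement follows control rotation with pitch zeroed.
; MainAttack press is forwarded to the possessed BP_FPSCharacter.
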(event EventTick
  (params (DeltaSeconds :type Float%20%28single-precision%29))
  (bind _returnvalue (Input|AxisValues|GetTurnRightRate))
  (bind _returnvalue_2 (Input|AxisValues|GetLookUpRate))
  (bind _lookdeadzone (Variables|Default|GetLookDeadzone))
  (bind _result (CallFunction|CalculateCircularDeadzone (Math|Vector2D|MakeVector2D _returnvalue _returnvalue_2) _lookdeadzone true))
  (bind _returnvalue_3 (* _result DeltaSeconds))
  ;[1 1 1] Input Handling
  (CallFunction|AddInputRotation self (Math|Rotator|MakeRotator (.y _returnvalue_3) 0.0 (.x _returnvalue_3)))
  (CallFunction|AddInputtoPawn (CallFunction|CalculateCircularDeadzone (Math|Vector2D|MakeVector2D (Input|AxisValues|GetMoveRight) (Input|AxisValues|GetMoveForward)) (Variables|Default|GetMoveDeadzone) true)))

(event Input|ActionEvents|InputActionMainAttack
  (:Pressed
    (bind _asbp_fpscharacter (Utilities|Casting|CastToBP_FPSCharacter (Pawn|GetControlledPawn)))
    (Default|CallMainAttackEvent _asbp_fpscharacter)))

(event Input|AxisEvents|InputAxisLookUp
  (params (AxisValue :type Float%20%28single-precision%29))
  ;[1 1 1] Input Handling
  (Class|PlayerController|AddPitchInput AxisValue))

(event Input|AxisEvents|InputAxisTurnRight
  (params (AxisValue :type Float%20%28single-precision%29))
  ;[1 1 1] Input Handling
  (Class|PlayerController|AddYawInput AxisValue))

(fn ConstructionScript)

(fn AddInputtoPawn
  (params (Input :type Vector%202D%20Structure))
  (bind _returnvalue (Pawn|GetControlRotation :!class /Script/Engine.Controller))
  (bind _returnvalue_2 (Pawn|GetControlledPawn))
  (bind _returnvalue_3 (Class|KismetMathLibrary|MakeRot 0.0 (.yaw _returnvalue) (.roll _returnvalue)))
  (Pawn|Input|AddMovementInput _returnvalue_2 (Math|Vector|GetForwardVector _returnvalue_3) (.y Input) false)
  (Pawn|Input|AddMovementInput _returnvalue_2 (Math|Vector|GetRightVector _returnvalue_3) (.x Input) false))